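; FinalTrigger1 is a quest trigger box that plays a scripted "To be continued" ending when overlapped.
; Its overlap event chains timed comment widgets with delays, showing Turkish dialogue before the closing message.
; The first comment appears for any overlapping actor; the rest requires MainCharacter, whose health is set to 1 as a fire sound plays.
; The character's UI widget is removed before the final message.
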(event `self.Box.OnComponentBeginOverlap`
  (params (OverlappedComponent :type "PrimitiveComponent Object Reference") (OtherActor :type "Actor Object Reference") (OtherComp :type "PrimitiveComponent Object Reference") (OtherBodyIndex :type Integer) (bFromSweep :type Boolean) (SweepResult :type "HitResult Structure (by ref)"))
  (bind _returnvalue (`|CreateWidget` "/Game/Widgets/Comment1.Comment1_C" null "BU DA NE?"))
  (`UserWidget.AddToViewport` _returnvalue 0)
  (`KismetSystemLibrary.Delay` 1.0)
  (`Widget.RemoveFromParent` _returnvalue)
  (bind _returnvalue_2 (`|CreateWidget` "/Game/Widgets/Comment1.Comment1_C" null "SONUNDA BİR DENEYİN DAHA SONUNA GELDİK"))
  (bind _asmain_character (cast `/Game/MainCharacter/BluePrints/MainCharacter` OtherActor))
  (`GameplayStatics.PlaySoundAtLocation` "/Game/SFX/Fire/Fire.Fire" (`self.K2_GetActorLocation` _asmain_character) (struct) 1.0 1.0 0.0 null null null)
  (set `/Game/MainCharacter/BluePrints/MainCharacter.CurrentHealth` 1.0 _asmain_character)
  (`UserWidget.AddToViewport` _returnvalue_2 0)
  (`KismetSystemLibrary.Delay` 2.0)
  (`Widget.RemoveFromParent` _returnvalue_2)
  (bind _asmain_character_2 (cast `/Game/MainCharacter/BluePrints/MainCharacter` OtherActor))
  (`Widget.RemoveFromParent` (`/Game/MainCharacter/BluePrints/MainCharacter.UI_Widget` _asmain_character_2))
  (bind _returnvalue_3 (`|CreateWidget` "/Game/Widgets/Comment.Comment_C" null "To be contunied"))
  (`UserWidget.AddToViewport` _returnvalue_3 0)
  (`KismetSystemLibrary.Delay` 2.0)
  (`Widget.RemoveFromParent` _returnvalue_3))

(fn `UserConstructionScript`)