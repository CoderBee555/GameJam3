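; Quest marker trigger that sends and removes quest messages through BPI_Quest when a qualifying actor overlaps its box.
; If a prerequisite is required, it searches the main character's quest panel widgets for it, then swaps it for the new quest once.
; Otherwise, every qualifying overlap sends the quest.
; Tick polls the listed target actors, intending to remove the sent quest once all are destroyed.
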(event `self.Box.OnComponentBeginOverlap`
  (params (OverlappedComponent :type "PrimitiveComponent Object Reference") (OtherActor :type "Actor Object Reference") (OtherComp :type "PrimitiveComponent Object Reference") (OtherBodyIndex :type Integer) (bFromSweep :type Boolean) (SweepResult :type "HitResult Structure (by ref)"))
  (if (`KismetSystemLibrary.DoesImplementInterface` OtherActor "/Game/Blueprints/Quests/BPI_Quest.BPI_Quest_C")
    (set `self.Quest Owner` OtherActor)
    (if (`self.NeedASpecificQuest?`)
      (bind _has_quest_ (`self.DoesHaveTheQuest`))
      (if _has_quest_
        (`/Engine/EditorBlueprintResources/StandardMacros.DoOnce` false
          (:`Completed`
            (message `/Game/Blueprints/Quests/BPI_Quest.Remove Quest` (`self.Quest Owner`) (`self.ShouldHaveQuest`))
            (message `/Game/Blueprints/Quests/BPI_Quest.Send Quest` (`self.Quest Owner`) (`self.SendQuest`)))))
      (else
        (message `/Game/Blueprints/Quests/BPI_Quest.Send Quest` (`self.Quest Owner`) (`self.SendQuest`))))))

(event `self.ReceiveTick`
  (params (DeltaSeconds :type "Float (single-precision)"))
  (bind _success_ (`self.CheckIsActorsAlive`))
  (if _success_
    (message `/Game/Blueprints/Quests/BPI_Quest.Remove Quest` (`self.Quest Owner`) (`self.SendQuest`))))

(fn `CheckIsActorsAlive`
  (returns (`Success?` :type Boolean))
  (locals (`Local Bool` :type Boolean :default true))
  (for _array_element (`self.ActorsNeedToDestroyForGivenQuest`)
    (`/Engine/EditorBlueprintResources/StandardMacros.IsValid` _array_element
      (:`Is Valid`
        (set `local.Local Bool` false))))
  (return (`local.Local Bool`)))

(fn `DoesHaveTheQuest`
  (returns (`Has Quest?` :type Boolean))
  (locals (`Has the Quest` :type Boolean :default false))
  (bind _asmain_character (cast `/Game/MainCharacter/BluePrints/MainCharacter` (`self.Quest Owner`)))
  (for _array_element (`PanelWidget.GetAllChildren` (`/Game/Widgets/UI.QuestPanel` (`/Game/MainCharacter/BluePrints/MainCharacter.UI_Widget` _asmain_character)))
    (bind _asquest_texts (cast `/Game/Widgets/QuestWidgets/QuestTexts` _array_element))
    (if (`KismetTextLibrary.EqualEqual_TextText` (`/Game/Widgets/QuestWidgets/QuestTexts.Quest` _asquest_texts) (`self.ShouldHaveQuest`))
      (set `local.Has the Quest` true)
      (return (`local.Has the Quest`)))))

(fn `UserConstructionScript`)