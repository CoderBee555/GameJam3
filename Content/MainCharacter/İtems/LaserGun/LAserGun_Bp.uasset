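; Player-held laser gun that charges up, then fires a continuous BP_Laser beam until attack is released.
; Pressing attack spins the rotating part via a timeline with charge sound; after a three-second delay it spawns the beam attached to the Arrow, with looping audio.
; Tick catches an early release, cancelling the shot and blocking input for a three-second recharge.
; Releasing attack stops beam and loop sound and resets the DoOnce gates.
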(event `self.ReceiveTick`
  (params (DeltaSeconds :type "Float (single-precision)"))
  (bind _chargesound (`self.ChargeSound`))
  (`|ExecutionSequence`
    (:`then_0`
      (if (and (`self.isCharging`) (`self.isReleased`))
        (`/Engine/EditorBlueprintResources/StandardMacros.DoOnce` false :!label _label
          (:`Completed`
            (`/Engine/EditorBlueprintResources/StandardMacros.IsValid` _chargesound
              (:`Is Valid`
                (`ActorComponent.K2_DestroyComponent` _chargesound)
                (`self.Uncharge`)))))))
    (:`then_1`
      (if (`self.isShooting`)
        _))))

(event `Reset Uncharge`
  (goto _label :!via `Reset`))

(event `Attack Pressed`
  (params (Player :type "/Game/MainCharacter/BluePrints/MainCharacter Object Reference"))
  (bind _laser (`self.Laser`))
  (if (not (`self.isRecharging`))
    (set `self.isReleased` false)
    (`/Engine/EditorBlueprintResources/StandardMacros.DoOnce` false :!label _label_2
      (:`Completed`
        (`/Engine/EditorBlueprintResources/StandardMacros.IsValid` _laser
          (:`Is Valid`
            (`/Game/MainCharacter/İtems/LaserGun/LaserBeam/BP_Laser.Stop Laser` _laser)
            (`self.Charge Animation And Sound`)
            (if (`self.isShotCanceled`)
              (set `self.isShotCanceled` false)
              (else
                (`self.Shoot Sound`)
                (bind _returnvalue (`|SpawnActorFromClass` "/Game/MainCharacter/İtems/LaserGun/LaserBeam/BP_Laser.BP_Laser_C" (`KismetMathLibrary.MakeTransform` (0.0 0.0 0.0)) "Undefined" "OverrideRootScale" null Player null :!label _label_3))
                (bind _output_get (set `self.Laser` _returnvalue))
                (`self.K2_AttachToComponent` _output_get (`self.Arrow`) "None" "SnapToTarget" "SnapToTarget" "KeepRelative" true)
                (set `self.isShooting` true))))
          (:`Is Not Valid`
            (`self.Charge Animation And Sound`)
            (if (`self.isShotCanceled`)
              (set `self.isShotCanceled` false)
              (else
                (`self.Shoot Sound`)
                (goto _label_3)))))))))

(event `Attack Released`
  (bind _laser (`self.Laser`))
  (set `self.isShooting` false)
  (`self.Reset Uncharge`)
  (set `self.isReleased` true)
  (`self.Remove Looping Sound`)
  (`/Engine/EditorBlueprintResources/StandardMacros.IsValid` _laser
    (:`Is Valid`
      (`/Game/MainCharacter/İtems/LaserGun/LaserBeam/BP_Laser.Stop Laser` _laser)
      (goto _label_2 :!via `Reset`))
    (:`Is Not Valid`
      (goto _label_2 :!via `Reset`))))

(fn `Remove Looping Sound`
  (`/Engine/EditorBlueprintResources/StandardMacros.IsValid` (`self.LoopSound`)
    (:`Is Valid`
      (`ActorComponent.K2_DestroyComponent` (`self.LoopSound`))
      (`GameplayStatics.PlaySoundAtLocation` "/Game/SFX/Laser/LaserOut.LaserOut" (`self.K2_GetActorLocation`) (struct) 1.0 1.0 0.0 null null null))))

(fn `UserConstructionScript`)