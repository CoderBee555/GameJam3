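; BP_Laser is the laser gun's beam actor, tracing from the player's follow camera each tick to set the Niagara beam end.
; At or below 50% heat, hit damageable actors receive delayed damage messages.
; Above that, only overpowered beams send messages, with zero damage, to all damageable actors within explosion range of the impact.
; StopLaser deactivates the effects and scales the beam through a timeline before destroying the actor.
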(event `Stop Laser`
  (`/Engine/EditorBlueprintResources/StandardMacros.DoOnce` false
    (:`Completed`
      (`ActorComponent.Deactivate` (`self.LaserBeam`))
      (`ActorComponent.Deactivate` (`self.Weapon Effect`))
      (set `self.End` true)
      (bind (_direction _scale) (`Timeline|StopEffect` :!via `PlayFromStart`)
        (:`Update`
          (`FXSystemComponent.SetFloatParameter` (`self.LaserBeam`) "User.Scale" _scale))
        (:`Finished`
          (`self.K2_DestroyActor`))))))

(event `self.ReceiveTick`
  (params (DeltaSeconds :type "Float (single-precision)"))
  (bind _playercharacter (`self.PlayerCharacter`))
  (bind _playercharacter_2 (`self.PlayerCharacter`))
  (bind _followcamera (`/Game/MainCharacter/BluePrints/MainCharacter.FollowCamera` (`self.PlayerCharacter`)))
  (bind _returnvalue (`SceneComponent.GetForwardVector` _followcamera))
  (bind _returnvalue_2 (`SceneComponent.K2_GetComponentLocation` _followcamera))
  (bind _outhit (`KismetSystemLibrary.LineTraceSingle` (+ _returnvalue_2 (* _returnvalue 100.0)) (+ _returnvalue_2 (* _returnvalue (`self.Weapon Range`))) "TraceTypeQuery1"))
  (bind (_bblockinghit _binitialoverlap _time _distance _location _impactpoint _normal _impactnormal _physmat _hitactor _hitcomponent _hitbonename _hititem _faceindex _tracestart _traceend) (`GameplayStatics.BreakHitResult` _outhit))
  (`FXSystemComponent.SetVectorParameter` (`self.LaserBeam`) "User.BeamEnd" (`KismetMathLibrary.SelectVector` _impactpoint _traceend (`KismetSystemLibrary.IsValid` _hitcomponent)))
  (if (`KismetSystemLibrary.DoesImplementInterface` _hitactor "/Game/Blueprints/BPI_Damageable.BPI_Damageable_C")
    (if (> (* (/ (`/Game/MainCharacter/BluePrints/MainCharacter.CurrentHeat` _playercharacter_2) (`/Game/MainCharacter/BluePrints/MainCharacter.MaxHeat` _playercharacter_2)) 100.0) 50.0)
      (if (`self.isOverpowered`)
        (bind _outactors (`GameplayStatics.GetAllActorsWithInterface` "/Game/Blueprints/BPI_Damageable.BPI_Damageable_C"))
        (for _array_element _outactors
          (if (< (`KismetMathLibrary.Vector_Distance` (`self.K2_GetActorLocation` _array_element) _impactpoint) (`self.ExplosionRange`))
            (message `/Game/Blueprints/BPI_Damageable.CustomDamageEvent` _array_element 0.0))))
      (else
        (`KismetSystemLibrary.Delay` 0.1)
        (message `/Game/Blueprints/BPI_Damageable.CustomDamageEvent` _hitactor 5.0)))
    (elif (`self.isOverpowered`)
      (if (> (* (/ (`/Game/MainCharacter/BluePrints/MainCharacter.CurrentHeat` _playercharacter) (`/Game/MainCharacter/BluePrints/MainCharacter.MaxHeat` _playercharacter)) 100.0) 50.0)
        (bind _outactors_2 (`GameplayStatics.GetAllActorsWithInterface` "/Game/Blueprints/BPI_Damageable.BPI_Damageable_C"))
        (for _array_element_2 _outactors_2
          (if (< (`KismetMathLibrary.Vector_Distance` (`self.K2_GetActorLocation` _array_element_2) _impactpoint) (`self.ExplosionRange`))
            (message `/Game/Blueprints/BPI_Damageable.CustomDamageEvent` _array_element_2 0.0)))))))

(fn `UserConstructionScript`)