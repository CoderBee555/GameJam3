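; Interactive hinged door Blueprint that swings open and closed on alternating Interact calls.
; A FlipFlop saves the current root rotation and a target 90 degrees further in yaw, then plays a timeline that lerps between them.
; Closing reverses the same timeline at a faster play rate, and each direction plays its own sound at the door mesh.
; The OpenClose event is empty.
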(event `/Game/Blueprints/BPI_Interactable.Interact`
  (params (Player :type "/Game/MainCharacter/BluePrints/MainCharacter Object Reference"))
  (bind _returnvalue (`SceneComponent.K2_GetComponentLocation` (`self.Door`)))
  (bind _returnvalue_2 (`SceneComponent.K2_GetComponentRotation` (`self.DefaultSceneRoot`)))
  (`/Engine/EditorBlueprintResources/StandardMacros.FlipFlop`
    (:`A`
      (set `self.DoorRotation` _returnvalue_2)
      (set `self.OpenRotation` (`KismetMathLibrary.MakeRotator` (.roll _returnvalue_2) (.pitch _returnvalue_2) (+ (.yaw _returnvalue_2) 90.0)))
      (`TimelineComponent.SetPlayRate` (`self.DoortimeLine`) 1.0)
      (`GameplayStatics.PlaySoundAtLocation` "/Game/SFX/DoorSFX/door-1-open.door-1-open" _returnvalue (struct) 1.0 1.0 0.0 null null null)
      (bind (_direction _doorcurve) (`Timeline|DoorTimeLine` :!label _label)
        (:`Update`
          (`SceneComponent.K2_SetWorldRotation` (`self.DefaultSceneRoot`) (`KismetMathLibrary.RLerp` (`self.DoorRotation`) (`self.OpenRotation`) _doorcurve) false false))))
    (:`B`
      (`TimelineComponent.SetPlayRate` (`self.DoortimeLine`) 1.45)
      (`GameplayStatics.PlaySoundAtLocation` "/Game/SFX/DoorSFX/door-1-close.door-1-close" _returnvalue (struct) 1.0 1.0 0.0 null null null)
      (goto _label :!via `Reverse`))))

(event `OpenClose`)

(fn `UserConstructionScript`)