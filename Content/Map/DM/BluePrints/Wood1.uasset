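; Destructible wood prop, apparently a tree, that breaks apart when its custom damage event fires and leaves a root mesh behind.
; The construction script and BeginPlay show the intact static mesh on a FakeMesh component.
; The damage event runs once, clearing that mesh, assigning the destructible mesh, pushing it with a fixed sideways force and setting the tree root mesh on Root.
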(event `self.ReceiveBeginPlay`
  (`/Engine/EditorBlueprintResources/StandardMacros.DoOnce` false
    (:`Completed`
      (`self.Set Static Mesh`))))

(event `/Game/Blueprints/BPI_Damageable.CustomDamageEvent`
  (params (DamageAmount :type "Float (single-precision)"))
  (`/Engine/EditorBlueprintResources/StandardMacros.DoOnce` false
    (:`Completed`
      (`self.Unset Static Mesh`)
      (`self.Set Destructible Mesh`)
      (`self.Destroy The Destructible Mesh`)
      (`StaticMeshComponent.SetStaticMesh` (`self.Root`) "/Game/Map/Tree/Root/TreeRoot.TreeRoot"))))

(fn `Destroy The Destructible Mesh`
  (`PrimitiveComponent.AddForce` (`self.Mesh`) (0.0 10000.0 0.0) "None" false))

(fn `Set Destructible Mesh`
  (`DestructibleComponent.SetDestructibleMesh` (`self.Mesh`) (`self.Destructible Mesh`)))

(fn `Set Static Mesh`
  (`StaticMeshComponent.SetStaticMesh` (`self.Fake Mesh`) (`self.Static Mesh`)))

(fn `Unset Static Mesh`
  (`StaticMeshComponent.SetStaticMesh` (`self.Fake Mesh`) null))

(fn `UserConstructionScript`
  (`StaticMeshComponent.SetStaticMesh` (`self.Fake Mesh`) (`self.Static Mesh`)))